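; Trigger actor that grants an ability asset to a character, with in-world text showing the ability and its load state.
; Construction script labels it with the name part of the ability's primary asset ID, or NULL if invalid.
; Load events switch the loading text from red "Loading.." to a green loaded-asset name.
; The grant event passes the loaded asset to the character through SetAbilityAsset.
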(event `self.OnAbilityLoadStart`
  (`TextRenderComponent.SetTextRenderColor` (`self.LoadingText`) (`KismetMathLibrary.Conv_LinearColorToColor` (struct :`R` 1.0 :`A` 1.0)))
  (`TextRenderComponent.SetTextRenderColor` (`self.AbilityText`) (`KismetMathLibrary.Conv_LinearColorToColor` (struct :`R` 1.0 :`A` 1.0)))
  (`TextRenderComponent.K2_SetText` (`self.LoadingText`) "Loading.."))

(event `self.BP_OnAbilityLoaded`
  (`TextRenderComponent.K2_SetText` (`self.LoadingText`) (`|FormatText` "Loaded: \n{Asset}" (`KismetSystemLibrary.GetObjectName` (`self.GetAbilityAsset`))))
  (`TextRenderComponent.SetTextRenderColor` (`self.LoadingText`) (`KismetMathLibrary.Conv_LinearColorToColor` (struct :`G` 1.0 :`A` 1.0))))

(event `self.GrantAbilityToCharacter`
  (params (Character :type "NotGDC_Character Object Reference"))
  (`NotGDC_Character.SetAbilityAsset` Character (`self.GetAbilityAsset`)))

(fn `UserConstructionScript`
  (`TextRenderComponent.K2_SetText` (`self.AbilityText`) (`|FormatText` "Ability: \n{Ability}" (select `bool` (`KismetSystemLibrary.IsValidPrimaryAssetId` (`self.GetAbilityId`)) :`false` "NULL" :`true` (`.RightS` (`KismetStringLibrary.Split` (`KismetSystemLibrary.Conv_PrimaryAssetIdToString` (`self.GetAbilityId`)) ":"))))))